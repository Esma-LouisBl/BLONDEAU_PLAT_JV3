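; BP_MovingWall is a platform actor that starts moving back and forth on BeginPlay and loops continuously.
; Two timelines, Move and MoveReverse, alternate with a one-second pause after each finishes.
; A MoveInX flag selects whether it travels along world X or Y.
; Each update adds the timeline's Position to the current location, so the value acts as a cumulative per-tick step, making travel distance frame-rate dependent.
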(event EventBeginPlay
  (bind _returnvalue (Transformation|GetActorLocation))
  (bind _returnvalue_2 (Transformation|GetActorLocation))
  (bind _returnvalue_3 (Transformation|GetActorLocation))
  (bind _returnvalue_4 (Transformation|GetActorLocation))
  (bind (_x _y _z) (Math|Vector|BreakVector _returnvalue))
  (bind (_x_2 _y_2 _z_2) (Math|Vector|BreakVector _returnvalue_2))
  (bind (_x_3 _y_3 _z_3) (Math|Vector|BreakVector _returnvalue_3))
  (bind (_x_4 _y_4 _z_4) (Math|Vector|BreakVector _returnvalue_4))
  (bind _position (Timeline|Move Play)
    (:Update
      (if (Variables|Default|GetMoveInX)
        (Transformation|SetActorLocation (Math|Vector|MakeVector (+ _position _x_2) _y_2 _z_2) false false)
        (else
          (Transformation|SetActorLocation (Math|Vector|MakeVector _x (+ _position _y) _z) false false))))
    (:Finished
      (Utilities|FlowControl|Delay 1.0)
      (bind _position_2 (Timeline|MoveReverse PlayFromStart)
        (:Update
          (if (Variables|Default|GetMoveInX)
            (Transformation|SetActorLocation (Math|Vector|MakeVector (+ _position_2 _x_3) _y_3 _z_3) false false)
            (else
              (Transformation|SetActorLocation (Math|Vector|MakeVector _x_4 (+ _position_2 _y_4) _z_4) false false))))
        (:Finished
          (Utilities|FlowControl|Delay 1.0)
          (Timeline|Move PlayFromStart))))))

(fn ConstructionScript)