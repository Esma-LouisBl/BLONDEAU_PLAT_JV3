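; BP_DashChargerGenerator spawns a BP_DashCharger pickup at its collision location when the third-person character overlaps it, keeping one tracked at a time.
; Each charger receives a reference back to the generator, whose DashCollected event clears the slot.
; A delayed loop rechecks after each spawn, respawning only if the slot is empty and the character remains inside, and otherwise ending until another overlap.
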(event OnComponentBeginOverlap(Collision)
  (params (OverlappedComponent :type Primitive%20Component%20Object%20Reference) (OtherActor :type Actor%20Object%20Reference) (OtherComp :type Primitive%20Component%20Object%20Reference) (OtherBodyIndex :type Integer) (bFromSweep :type Boolean) (SweepResult :type Hit%20Result%20Structure%20%28by%20ref%29))
  (Utilities|Casting|CastToBP_ThirdPersonCharacter OtherActor)
  (Variables|Default|SetCanGenerate true)
  (if (Variables|Default|GetCanGenerate) :!label _label
    (if (== (Variables|Default|GetDash%20Charger) 0)
      (bind _returnvalue (Game|SpawnActorfromClass "/Game/Blueprints/Collectables/BP_DashCharger.BP_DashCharger_C" (Math|Transform|MakeTransform (Transformation|GetWorldLocation (Variables|Default|GetCollision)) "0, 0, 0" "1.000000,1.000000,1.000000") "Undefined" "MultiplyWithRoot" 0 0 0))
      (Utilities|IsValid _returnvalue
        (:Is%20Valid
          (Variables|/Game/Blueprints/Collectables/BP_DashCharger.BP_DashCharger_C|SetGenerator _returnvalue self)
          (Variables|Default|SetDash%20Charger _returnvalue)
          (Utilities|FlowControl|Delay 3.0)
          (goto _label))))))

(event OnComponentEndOverlap(Collision)
  (params (OverlappedComponent :type Primitive%20Component%20Object%20Reference) (OtherActor :type Actor%20Object%20Reference) (OtherComp :type Primitive%20Component%20Object%20Reference) (OtherBodyIndex :type Integer))
  (Utilities|Casting|CastToBP_ThirdPersonCharacter OtherActor)
  (Variables|Default|SetCanGenerate false))

(event Custom|Dash%20Collected
  (Variables|Default|SetDash%20Charger 0))

(fn ConstructionScript)